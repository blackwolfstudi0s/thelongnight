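; Explosive barrel actor that blows up when shot by a rifle, pistol or shotgun projectile.
; Its Box overlap checks the other actor's projectile tag, then destroys the barrel and plays an explosion sound and enlarged rocket launcher particle effect at its location.
; Nested overlap checks on three radius components outline distance-based damage, but their branches lead to no action, so no damage is applied.
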(event `self.Box.OnComponentBeginOverlap`
  (params (OverlappedComponent :type "PrimitiveComponent Object Reference") (OtherActor :type "Actor Object Reference") (OtherComp :type "PrimitiveComponent Object Reference") (OtherBodyIndex :type Integer) (bFromSweep :type Boolean) (SweepResult :type "HitResult Structure (by ref)"))
  (bind _returnvalue (`self.K2_GetActorLocation`))
  ;[1 1 1] Barrel can only be shot
  (if (`self.ActorHasTag` OtherActor "Tag_Projectile_Rifle")
    (`self.K2_DestroyActor` :!label _label)
    (`GameplayStatics.PlaySoundAtLocation` "/Game/StarterContent/Audio/Explosion01.Explosion01" _returnvalue (struct) 1.0 1.0 0.0 null null null)
    (`GameplayStatics.SpawnEmitterAtLocation` "/Game/__MyContent_Luke/_Lukes_content/MilitaryWeapDark/FX/P_RocketLauncher_Explosion_01.P_RocketLauncher_Explosion_01" _returnvalue (struct) (2.0 2.0 2.0))
    ;[1 1 1] Damage overlap within radias
    (if (`PrimitiveComponent.IsOverlappingComponent` (`self.inner inner radius`) null)
      _
      (elif (`PrimitiveComponent.IsOverlappingComponent` (`self.inner radius`) null)
        _
        (elif (`PrimitiveComponent.IsOverlappingActor` (`self.damage radius`) null)
          _)))
    (elif (`self.ActorHasTag` OtherActor "Tag_Projectile_Pistol")
      (goto _label)
      (elif (`self.ActorHasTag` OtherActor "Tag_Projectile_Shotgun")
        (goto _label)))))

(fn `UserConstructionScript`)