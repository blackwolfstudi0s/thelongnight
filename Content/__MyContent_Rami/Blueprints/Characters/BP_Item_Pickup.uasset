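; Collectible item pickup actor for weapons, ammo, health, an hour glass or a key, chosen by its ItemPickup type.
; The construction script swaps the Pickup mesh to match that type, and Tick spins the actor slowly each frame by a fixed, frame-rate-dependent step.
; When an actor tagged as the player overlaps the mesh, it passes the type to the game manager's CollectPickup and destroys itself.
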(event `self.ReceiveTick`
  (params (DeltaSeconds :type "Float (single-precision)"))
  (`self.K2_SetActorRotation` (`KismetMathLibrary.ComposeRotators` (`self.K2_GetActorRotation`) (struct :`Yaw` 3.0))))

(event `self.Pickup.OnComponentBeginOverlap`
  (params (OverlappedComponent :type "PrimitiveComponent Object Reference") (OtherActor :type "Actor Object Reference") (OtherComp :type "PrimitiveComponent Object Reference") (OtherBodyIndex :type Integer) (bFromSweep :type Boolean) (SweepResult :type "HitResult Structure (by ref)"))
  (if (`self.ActorHasTag` OtherActor "Tag_Player")
    (bind _game_manager (`/Game/__MyContent_Rami/Blueprints/BP_FunctionLibrary.Get Game Manager`))
    (`/Game/__MyContent_Rami/Blueprints/BP_GameManager.Collect Pickup` _game_manager (`self.ItemPickup`))
    (`self.K2_DestroyActor`)))

(fn `UserConstructionScript`
  (bind _pickup (`self.Pickup`))
  (switch `/Game/__MyContent_Rami/Blueprints/Enums/BP_ItemPickup` (`self.ItemPickup`)
    (:`NewEnumerator1`
      (`StaticMeshComponent.SetStaticMesh` _pickup "/Game/__MyContent_Rami/Meshes/Pistol_Mesh.Pistol_Mesh"))
    (:`NewEnumerator0`
      (`StaticMeshComponent.SetStaticMesh` _pickup "/Game/__MyContent_Rami/Meshes/Assault_Rifle_Mesh.Assault_Rifle_Mesh"))
    (:`NewEnumerator2`
      (`StaticMeshComponent.SetStaticMesh` _pickup "/Game/__MyContent_Rami/Meshes/Shotgun_Mesh.Shotgun_Mesh"))
    (:`NewEnumerator3`
      (`StaticMeshComponent.SetStaticMesh` _pickup "/Game/__MyContent_Rami/Meshes/Ammo_Pickup_Mesh.Ammo_Pickup_Mesh"))
    (:`NewEnumerator4`
      (`StaticMeshComponent.SetStaticMesh` _pickup "/Game/__MyContent_Rami/Meshes/Health_Pickup_Mesh.Health_Pickup_Mesh"))
    (:`NewEnumerator5`
      (`StaticMeshComponent.SetStaticMesh` _pickup "/Game/__MyContent_Rami/Meshes/Hour_Glass_Mesh.Hour_Glass_Mesh"))
    (:`NewEnumerator6`
      (`StaticMeshComponent.SetStaticMesh` _pickup "/Game/__MyContent_Rami/Meshes/Key_Mesh.Key_Mesh"))))