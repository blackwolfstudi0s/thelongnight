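; BP_EnemySpawn is a spawner that creates a batch of BP_EnemyZombie AI pawns at its Sphere component when play begins.
; Each spawned zombie receives the spawner's ZombieType and MiniBoss settings, then a skin matching that type: skinny, average, fat or dog.
; Nested FlipFlops alternate skin variants across successive spawns for variety, while dogs always use one wolf mesh.
; The construction script caps SpawnQuantity at 30.
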(event `self.ReceiveBeginPlay`
  (for _ (range 1 (+ (`self.Spawn Quantity`) 1))
    (`self.Spawn Zombie`)))

(event `Spawn Zombie`
  (bind _sphere (`self.Sphere`))
  (bind _zombie_type (`self.Zombie Type`))
  (bind _returnvalue (`AIBlueprintHelperLibrary.SpawnAIFromClass` "/Game/__MyContent_Rami/Blueprints/Characters/BP_EnemyZombie.BP_EnemyZombie_C" null (`SceneComponent.K2_GetComponentLocation` _sphere) (`SceneComponent.K2_GetComponentRotation` _sphere)))
  (bind _asbp_enemy_zombie (cast `/Game/__MyContent_Rami/Blueprints/Characters/BP_EnemyZombie` _returnvalue))
  (`/Game/__MyContent_Rami/Blueprints/Characters/BP_EnemyZombie.Set Parameters` _asbp_enemy_zombie _zombie_type (`self.Mini-Boss`))
  (switch `/Game/__MyContent_Rami/Blueprints/Enums/BP_ZombieTypes` _zombie_type
    (:`NewEnumerator0`
      (`/Engine/EditorBlueprintResources/StandardMacros.FlipFlop`
        (:`A`
          (`/Game/__MyContent_Rami/Blueprints/Characters/BP_EnemyZombie.Set Skin` _asbp_enemy_zombie "/Game/__MyContent_Rami/Packs/ZombieMeshes/SK_ZombieAD_1.SK_ZombieAD_1"))
        (:`B`
          (`/Engine/EditorBlueprintResources/StandardMacros.FlipFlop`
            (:`A`
              (`/Game/__MyContent_Rami/Blueprints/Characters/BP_EnemyZombie.Set Skin` _asbp_enemy_zombie "/Game/__MyContent_Rami/Packs/ZombieMeshes/SK_ZombieAE_1.SK_ZombieAE_1"))
            (:`B`
              (`/Game/__MyContent_Rami/Blueprints/Characters/BP_EnemyZombie.Set Skin` _asbp_enemy_zombie "/Game/__MyContent_Rami/Packs/ZombieMeshes/SK_ZombieAE_2.SK_ZombieAE_2"))))))
    (:`NewEnumerator1`
      (`/Engine/EditorBlueprintResources/StandardMacros.FlipFlop`
        (:`A`
          (`/Engine/EditorBlueprintResources/StandardMacros.FlipFlop`
            (:`A`
              (`/Game/__MyContent_Rami/Blueprints/Characters/BP_EnemyZombie.Set Skin` _asbp_enemy_zombie "/Game/__MyContent_Rami/Packs/ZombieMeshes/SK_ZombieAC_1.SK_ZombieAC_1"))
            (:`B`
              (`/Game/__MyContent_Rami/Blueprints/Characters/BP_EnemyZombie.Set Skin` _asbp_enemy_zombie "/Game/__MyContent_Rami/Packs/ZombieMeshes/SK_ZombieAC_2.SK_ZombieAC_2"))))
        (:`B`
          (`/Engine/EditorBlueprintResources/StandardMacros.FlipFlop`
            (:`A`
              (`/Game/__MyContent_Rami/Blueprints/Characters/BP_EnemyZombie.Set Skin` _asbp_enemy_zombie "/Game/__MyContent_Rami/Packs/ZombieMeshes/SK_ZombieAA_1.SK_ZombieAA_1"))
            (:`B`
              (`/Game/__MyContent_Rami/Blueprints/Characters/BP_EnemyZombie.Set Skin` _asbp_enemy_zombie "/Game/__MyContent_Rami/Packs/ZombieMeshes/SK_ZombieAA_3.SK_ZombieAA_3"))))))
    (:`NewEnumerator2`
      (`/Engine/EditorBlueprintResources/StandardMacros.FlipFlop`
        (:`A`
          (`/Game/__MyContent_Rami/Blueprints/Characters/BP_EnemyZombie.Set Skin` _asbp_enemy_zombie "/Game/__MyContent_Rami/Packs/ZombieMeshes/SK_ZombieAB_1.SK_ZombieAB_1"))
        (:`B`
          (`/Engine/EditorBlueprintResources/StandardMacros.FlipFlop`
            (:`A`
              (`/Game/__MyContent_Rami/Blueprints/Characters/BP_EnemyZombie.Set Skin` _asbp_enemy_zombie "/Game/__MyContent_Rami/Packs/ZombieMeshes/SK_ZombieAB_2.SK_ZombieAB_2"))
            (:`B`
              (`/Game/__MyContent_Rami/Blueprints/Characters/BP_EnemyZombie.Set Skin` _asbp_enemy_zombie "/Game/__MyContent_Rami/Packs/ZombieMeshes/SK_ZombieAB_3.SK_ZombieAB_3"))))))
    (:`NewEnumerator5`
      (`/Game/__MyContent_Rami/Blueprints/Characters/BP_EnemyZombie.Set Skin` _asbp_enemy_zombie "/Game/__MyContent_Rami/Packs/ZombieMeshes/SK_Wolf_2.SK_Wolf_2"))))

(fn `UserConstructionScript`
  (if (> (`self.Spawn Quantity`) 30)
    (set `self.Spawn Quantity` 30)))