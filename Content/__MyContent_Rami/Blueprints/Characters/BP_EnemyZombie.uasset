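; Enemy character for skinny, average, fat and dog zombies, configured by SetParameters, with an optional scaled-up miniboss variant.
; Tick detects the player by distance or prior damage, then chases with MoveToLocation or damages them repeatedly through the game manager.
; Tagged projectile overlaps reduce health, with shotgun pellets losing penetration by zombie type.
; Death awards points, shows a blood decal and spawns a pickup, guaranteed for minibosses, random otherwise.
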(event `Play Zombie Sound`
  (bind _zombiesound (`self.ZombieSound`))
  (bind _zombiesound_2 (`self.ZombieSound`))
  ;[1 1 1] Play Zombie Sound
  (`/Engine/EditorBlueprintResources/StandardMacros.DoOnce` false
    (:`Completed`
      (if (`|EnumInequality` (`self.Zombie Type`) "NewEnumerator5")
        (if (not (`self.IsDead`)) :!label _label
          (`AudioComponent.FadeIn` _zombiesound_2 0.25 1.0 (`KismetMathLibrary.RandomFloatInRange` 0.0 103.0))
          (`KismetSystemLibrary.Delay` (`KismetMathLibrary.RandomFloatInRange` 4.0 8.0))
          (`AudioComponent.FadeOut` _zombiesound 1.0 0.0)
          (`KismetSystemLibrary.Delay` 1.0)
          (`AudioComponent.Stop` _zombiesound)
          (`KismetSystemLibrary.Delay` (`KismetMathLibrary.RandomFloatInRange` 0.5 2.0))
          (goto _label)
          (else
            (`AudioComponent.Stop` _zombiesound_2)))
        (else
          (`AudioComponent.Play` (`self.ZombieSound`) (`KismetMathLibrary.RandomFloatInRange` 0.0 6.0)))))))

(event `self.ReceiveTick`
  (params (DeltaSeconds :type "Float (single-precision)"))
  ;[1 1 1] Enemy AI moving and attacking
  (if (or (<= (`self.GetDistanceTo` (`/Game/__MyContent_Rami/Blueprints/Game/BP_FunctionLibrary.Get Player`)) (`self.DetectedDistance`)) (`self.IsDetected`))
    (`self.Play Zombie Sound`)
    (bind _output_get (set `self.IsDetected` true))
    (if _output_get
      (if (and (<= (`self.GetDistanceTo` (`/Game/__MyContent_Rami/Blueprints/Game/BP_FunctionLibrary.Get Player`)) (`self.AttackDistance`)) (not (`self.IsDead`)))
        (if (not (`self.IsAttacking`))
          (set `self.IsAttacking` true)
          (`self.K2_SetActorRotation` (`KismetMathLibrary.FindLookAtRotation` (`self.K2_GetActorLocation`) (`self.K2_GetActorLocation` (`/Game/__MyContent_Rami/Blueprints/Game/BP_FunctionLibrary.Get Player`))))
          (`self.Modify Zombie Mouth` false true true)
          (if (`self.IsAttacking`) :!label _label_2
            (`/Game/__MyContent_Rami/Blueprints/Game/BP_GameManager.Damage Player` (`/Game/__MyContent_Rami/Blueprints/Game/BP_FunctionLibrary.Get Game Manager`) (`self.Zombie Type`) (`self.Mini-Boss`))
            (`KismetSystemLibrary.Delay` 0.15)
            (goto _label_2)))
        (else
          (set `self.IsAttacking` false)
          (if (and (`self.IsDetected`) (not (`self.IsDead`)))
            (`self.Modify Zombie Mouth` false true)
            (`AIController.MoveToLocation` (`AIBlueprintHelperLibrary.GetAIController` self) (`self.K2_GetActorLocation` (`/Game/__MyContent_Rami/Blueprints/Game/BP_FunctionLibrary.Get Player`)) (`self.AttackDistance`) false true false true null false)))))))

(event `self.Mesh.OnComponentBeginOverlap`
  (params (OverlappedComponent :type "PrimitiveComponent Object Reference") (OtherActor :type "Actor Object Reference") (OtherComp :type "PrimitiveComponent Object Reference") (OtherBodyIndex :type Integer) (bFromSweep :type Boolean) (SweepResult :type "HitResult Structure (by ref)"))
  ;[1 1 1] Bullet Hits Zombie
  (if (not (`self.IsDead`))
    (if (`self.ActorHasTag` OtherActor "Tag_Projectile_Rifle")
      (`self.K2_DestroyActor` OtherActor)
      (set `self.Shotgun` false)
      (`self.Set Health` -50.0)
      (elif (`self.ActorHasTag` OtherActor "Tag_Projectile_Pistol")
        (`self.K2_DestroyActor` OtherActor)
        (set `self.Shotgun` false)
        (`self.Set Health` -50.0)
        (elif (`self.ActorHasTag` OtherActor "Tag_Projectile_Shotgun")
          (set `self.Shotgun` true)
          (bind _asbp_projectile_shotgun (cast `/Game/__MyContent_Rami/Blueprints/Projectiles/BP_Projectile_Shotgun` OtherActor))
          (switch `/Game/__MyContent_Rami/Blueprints/Enums/BP_ZombieTypes` (`self.Zombie Type`)
            (:`NewEnumerator0`
              (`/Game/__MyContent_Rami/Blueprints/Projectiles/BP_Projectile_Shotgun.Set Bullet Health` _asbp_projectile_shotgun -50.0))
            (:`NewEnumerator1`
              (`/Game/__MyContent_Rami/Blueprints/Projectiles/BP_Projectile_Shotgun.Set Bullet Health` _asbp_projectile_shotgun -75.0))
            (:`NewEnumerator2`
              (`/Game/__MyContent_Rami/Blueprints/Projectiles/BP_Projectile_Shotgun.Set Bullet Health` _asbp_projectile_shotgun -150.0 :!label _label_3))
            (:`NewEnumerator5`
              (goto _label_3)))
          (if (<= (`/Game/__MyContent_Rami/Blueprints/Projectiles/BP_Projectile_Shotgun.Get Bullet Health` _asbp_projectile_shotgun) 0.0)
            (`self.K2_DestroyActor` _asbp_projectile_shotgun))
          (`self.Set Health` -25.0))))))

(event `CheckIsDead`
  (bind _capsulecomponent (`self.CapsuleComponent`))
  (bind _decal (`self.Decal`))
  ;[1 1 1] Death Sequence
  (if (<= (`self.ZombieHealth`) 0.0)
    (set `self.IsAttacking` false)
    (`/Engine/EditorBlueprintResources/StandardMacros.DoOnce` false
      (:`Completed`
        (`PrimitiveComponent.SetCollisionResponseToChannel` _capsulecomponent "ECC_Pawn" "ECR_Overlap")
        (`PrimitiveComponent.SetCollisionResponseToChannel` _capsulecomponent "ECC_Visibility" "ECR_Ignore")
        (`self.Modify Zombie Mouth` true)
        (set `self.IsDead` true)
        (`AudioComponent.Stop` (`self.ZombieSound`))
        (`MovementComponent.StopMovementImmediately` (`self.CharacterMovement`))
        (`self.Increase Points`)
        (`SceneComponent.K2_SetWorldRotation` _decal (`KismetMathLibrary.MakeRotator` (`KismetMathLibrary.RandomFloatInRange` -180.0 180.0) -90.0) false false)
        (`SceneComponent.SetVisibility` _decal true false)
        (`DecalComponent.SetDecalMaterial` _decal (`|GetArrayItem` (`self.Blood Decals`) (`KismetMathLibrary.RandomInteger` 4)))
        (set `self.DeathLoc` (+ (`self.K2_GetActorLocation`) (0.0 0.0 0.0)))
        (if (`self.Mini-Boss`)
          (bind _returnvalue (`|SpawnActorFromClass` "/Game/BP_PlaceInWorld/BP_ItemPickup.BP_ItemPickup_C" (`KismetMathLibrary.MakeTransform` (`self.DeathLoc`)) "AdjustIfPossibleButAlwaysSpawn" "OverrideRootScale" null null))
          (`/Game/BP_PlaceInWorld/BP_ItemPickup.Set Item Type` _returnvalue "NewEnumerator6")
          (else
            (bind _output_get (set `self.DropChance` (`KismetMathLibrary.RandomInteger` 20)))
            (switch `int` _output_get
              (:`0`
                (bind _returnvalue_2 (`|SpawnActorFromClass` "/Game/BP_PlaceInWorld/BP_ItemPickup.BP_ItemPickup_C" (`KismetMathLibrary.MakeTransform` (`self.DeathLoc`)) "AdjustIfPossibleButAlwaysSpawn" "OverrideRootScale" null null))
                (`/Game/BP_PlaceInWorld/BP_ItemPickup.Set Item Type` _returnvalue_2 "NewEnumerator4"))
              (:`1`
                (bind _returnvalue_3 (`|SpawnActorFromClass` "/Game/BP_PlaceInWorld/BP_ItemPickup.BP_ItemPickup_C" (`KismetMathLibrary.MakeTransform` (`self.DeathLoc`)) "AdjustIfPossibleButAlwaysSpawn" "OverrideRootScale" null null :!label _label_4))
                (`/Game/BP_PlaceInWorld/BP_ItemPickup.Set Item Type` _returnvalue_3 "NewEnumerator3"))
              (:`2`
                (bind _returnvalue_4 (`|SpawnActorFromClass` "/Game/BP_PlaceInWorld/BP_ItemPickup.BP_ItemPickup_C" (`KismetMathLibrary.MakeTransform` (`self.DeathLoc`)) "AdjustIfPossibleButAlwaysSpawn" "OverrideRootScale" null null :!label _label_5))
                (`/Game/BP_PlaceInWorld/BP_ItemPickup.Set Item Type` _returnvalue_4 "NewEnumerator5"))
              (:`3`
                (goto _label_4))
              (:`4`
                (goto _label_5)))))))
    (else
      (set `self.IsDetected` true))))

(fn `Get Parameters Animation`
  (returns (`Zombie Type` :type "/Game/__MyContent_Rami/Blueprints/Enums/BP_ZombieTypes Enum") (Shotgun :type Boolean) (IsInjured :type Boolean) (IsDead :type Boolean) (IsAttacking :type Boolean))
  (return (`self.Zombie Type`) (`self.Shotgun`) (`self.IsInjured`) (`self.IsDead`) (`self.IsAttacking`)))

(fn `Increase Points`
  (switch `/Game/__MyContent_Rami/Blueprints/Enums/BP_ZombieTypes` (`self.Zombie Type`)
    (:`NewEnumerator0`
      (set `self.Score Points` 100))
    (:`NewEnumerator1`
      (set `self.Score Points` 200))
    (:`NewEnumerator2`
      (set `self.Score Points` 400 :!label _label))
    (:`NewEnumerator5`
      (goto _label)))
  (if (`self.Mini-Boss`)
    (set `self.Score Points` (* (`self.Score Points`) 2)))
  (`/Game/__MyContent_Rami/Blueprints/Game/BP_GameManager.Set Score` (`/Game/__MyContent_Rami/Blueprints/Game/BP_FunctionLibrary.Get Game Manager`) (`self.Score Points`)))

(fn `Modify Zombie Mouth`
  (params (Random :type Boolean) (Grin :type Boolean) (`Open Mouth` :type Boolean))
  (bind _mesh (`self.Mesh`))
  (bind _mesh_2 (`self.Mesh`))
  (if (`|EnumInequality` (`self.Zombie Type`) "NewEnumerator5")
    (if (`self.MouthEnabled`)
      (if Random
        (`SkeletalMeshComponent.SetMorphTarget` _mesh "ZombieGrin" (`KismetMathLibrary.Conv_IntToDouble` (`KismetMathLibrary.RandomIntegerInRange` 0 1)) true)
        (`SkeletalMeshComponent.SetMorphTarget` _mesh "ZombieOpenMouth" (`KismetMathLibrary.Conv_IntToDouble` (`KismetMathLibrary.RandomIntegerInRange` 0 1)) true)
        (else
          (if Grin
            (`SkeletalMeshComponent.SetMorphTarget` _mesh_2 "ZombieGrin" 1.0 true)
            (else
              (`SkeletalMeshComponent.SetMorphTarget` _mesh_2 "ZombieGrin" 0.0 true)))
          (if `Open Mouth`
            (`SkeletalMeshComponent.SetMorphTarget` (`self.Mesh`) "ZombieOpenMouth" 1.0 true)
            (else
              (`SkeletalMeshComponent.SetMorphTarget` (`self.Mesh`) "ZombieOpenMouth" 0.0 true))))))))

(fn `Set Attack Distance`
  (if (`|EnumInequality` (`self.Zombie Type`) "NewEnumerator5")
    (set `self.AttackDistance` 110.0)
    (else
      (set `self.AttackDistance` 150.0)))
  (if (`self.Mini-Boss`)
    (set `self.AttackDistance` (* (`self.AttackDistance`) 1.5))))

(fn `Set Health`
  (params (DeltaHealth :type "Float (double-precision)"))
  (set `self.ZombieHealth` (+ DeltaHealth (`self.ZombieHealth`)))
  (if (< DeltaHealth 0.0)
    (`self.CheckIsDead`)))

(fn `Set Parameters`
  (params (`Zombie Type` :type "/Game/__MyContent_Rami/Blueprints/Enums/BP_ZombieTypes Enum" :default "NewEnumerator0") (`Mini-Boss` :type Boolean))
  (bind _zombiesound (`self.ZombieSound`))
  (bind _mesh (`self.Mesh`))
  (bind _zombiesound_2 (`self.ZombieSound`))
  (bind _output_get (set `self.Zombie Type` `Zombie Type`))
  (bind _output_get_2 (set `self.Mini-Boss` `Mini-Boss`))
  (`self.Set Attack Distance`)
  (switch `/Game/__MyContent_Rami/Blueprints/Enums/BP_ZombieTypes` _output_get
    (:`NewEnumerator0`
      (`AudioComponent.SetPitchMultiplier` _zombiesound_2 1.3)
      (`self.Set Speed` 850.0)
      (`self.Set Health` 100.0)
      (`SkeletalMeshComponent.SetAnimInstanceClass` _mesh "/Game/__MyContent_Rami/Animations/ZombieAnimation.ZombieAnimation_C" :!label _label)
      (`AudioComponent.SetSound` _zombiesound "/Game/__MyContent_Rami/Audio/Zombie_Audio.Zombie_Audio"))
    (:`NewEnumerator1`
      (`AudioComponent.SetPitchMultiplier` _zombiesound_2 1.0)
      (`self.Set Speed` 625.0)
      (`self.Set Health` 200.0)
      (goto _label))
    (:`NewEnumerator2`
      (`AudioComponent.SetPitchMultiplier` _zombiesound_2 0.7)
      (`self.Set Speed` 400.0)
      (`self.Set Health` 400.0)
      (goto _label))
    (:`NewEnumerator5`
      (`self.Set Speed` 850.0)
      (`self.Set Health` 400.0)
      (`SkeletalMeshComponent.SetAnimInstanceClass` _mesh "/Game/__MyContent_Rami/Animations/DogAnimation.DogAnimation_C")
      (`AudioComponent.SetSound` _zombiesound "/Game/__MyContent_Rami/Audio/Zombie_Dog.Zombie_Dog")))
  (if _output_get_2
    (`SceneComponent.SetWorldScale3D` (`self.CapsuleComponent`) (1.5 1.5 1.5))
    (set `self.ZombieHealth` (* (`self.ZombieHealth`) 4.0))
    (`AudioComponent.SetVolumeMultiplier` (`self.ZombieSound`) 2.0)))

(fn `Set Skin`
  (params (NewMesh :type "SkeletalMesh Object Reference"))
  (`SkinnedMeshComponent.SetSkinnedAssetAndUpdate` (`self.Mesh`) NewMesh true))

(fn `Set Speed`
  (params (`Run Speed` :type "Float (double-precision)"))
  (set `CharacterMovementComponent.MaxWalkSpeed` `Run Speed` (`self.CharacterMovement`)))

(fn `UserConstructionScript`)