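; BP_SaveCheckpoint is a checkpoint actor that saves the game when the player enters it.
; When an actor tagged Tag_Player overlaps its CheckpointSave component, it registers itself as the player's checkpoint and calls SaveGame on the game manager.
; It skips saving if it is already the player's current checkpoint.
; On BeginPlay it disables its collision and re-enables it after a short delay.
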(event `self.ReceiveBeginPlay`
  (`self.SetActorEnableCollision` false)
  (`KismetSystemLibrary.Delay` 0.1)
  (`self.SetActorEnableCollision` true))

(event `self.CheckpointSave.OnComponentBeginOverlap`
  (params (OverlappedComponent :type "PrimitiveComponent Object Reference") (OtherActor :type "Actor Object Reference") (OtherComp :type "PrimitiveComponent Object Reference") (OtherBodyIndex :type Integer) (bFromSweep :type Boolean) (SweepResult :type "HitResult Structure (by ref)"))
  (if (and (`self.ActorHasTag` OtherActor "Tag_Player") (!= self (`/Game/__MyContent_Rami/Blueprints/Characters/BP_FirstPersonPlayer.GetSaveCheckpoint` (`/Game/__MyContent_Rami/Blueprints/BP_FunctionLibrary.Get Player`))))
    (`/Game/__MyContent_Rami/Blueprints/Characters/BP_FirstPersonPlayer.SetSaveCheckpoint` (`/Game/__MyContent_Rami/Blueprints/BP_FunctionLibrary.Get Player`) self)
    (`/Game/__MyContent_Rami/Blueprints/BP_GameManager.SaveGame` (`/Game/__MyContent_Rami/Blueprints/BP_FunctionLibrary.Get Game Manager`))))

(fn `UserConstructionScript`)