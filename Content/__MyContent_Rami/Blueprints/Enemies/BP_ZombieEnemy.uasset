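; Zombie enemy character (skinny, average, fat or dog, optionally a mini-boss) that chases and damages the player and awards score on death.
; A looping timer drives AI MoveTo once detection or a bullet hit alerts it, and repeats melee damage through the GameManager when close.
; Tagged projectile overlaps reduce health and flash its lights red.
; SetParameters configures each variant, with morph targets animating the mouth and a random blood decal on death.
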(event `self.ReceiveBeginPlay`
  ;[1 1 1] Enemy AI moving and attacking
  (`self.Set Front Back Lights Intensity` (`self.High Light Intensity`))
  (`KismetSystemLibrary.K2_SetTimer` null "TrackPlayer" 0.1 true))

(event `TrackPlayer`
  ;[1 1 1] Enemy AI moving and attacking
  (bind _player (`/Game/__MyContent_Rami/Blueprints/BP_FunctionLibrary.Get Player`))
  (if (and (<= (`self.GetDistanceTo` _player) 100.0) (not (`self.IsDead`)))
    (if (not (`self.IsAttacking`))
      (set `self.IsAttacking` true)
      (bind _player_2 (`/Game/__MyContent_Rami/Blueprints/BP_FunctionLibrary.Get Player`))
      (`self.K2_SetActorRotation` (`KismetMathLibrary.FindLookAtRotation` (`self.K2_GetActorLocation`) (`self.K2_GetActorLocation` _player_2)))
      (`KismetSystemLibrary.Delay` 0.3)
      (`self.Change Zombie Mouth` false true true)
      (if (`self.IsAttacking`) :!label _label
        (bind _game_manager (`/Game/__MyContent_Rami/Blueprints/BP_FunctionLibrary.Get Game Manager`))
        (`/Game/__MyContent_Rami/Blueprints/BP_GameManager.Damage Player` _game_manager (`self.Zombie Type`) (`self.Mini-Boss`))
        (`KismetSystemLibrary.Delay` 0.25)
        (goto _label)))
    (else
      (set `self.IsAttacking` false)
      (if (and (`self.IsDetected`) (not (`self.IsDead`)))
        (`self.Change Zombie Mouth` false true)
        (bind _player_3 (`/Game/__MyContent_Rami/Blueprints/BP_FunctionLibrary.Get Player`))
        (`AIController.MoveToLocation` (`AIBlueprintHelperLibrary.GetAIController` self) (`self.K2_GetActorLocation` _player_3) 100.0 false true false true null false)))))

(event `self.Mesh.OnComponentBeginOverlap`
  (params (OverlappedComponent :type "PrimitiveComponent Object Reference") (OtherActor :type "Actor Object Reference") (OtherComp :type "PrimitiveComponent Object Reference") (OtherBodyIndex :type Integer) (bFromSweep :type Boolean) (SweepResult :type "HitResult Structure (by ref)"))
  (bind _decal (`self.Decal`))
  ;[1 1 1] Bullets Hits Zombie
  (if (`self.ActorHasTag` OtherActor "Tag_Projectile_Rifle")
    (set `self.ZombieHealth` (- (`self.ZombieHealth`) 20.0))
    (`self.K2_DestroyActor` OtherActor :!label _label_2)
    (if (<= (`self.ZombieHealth`) 0.0) :!label _label_3
      (`self.FlashRed`)
      (`KismetSystemLibrary.Delay` 0.1)
      (set `self.IsAttacking` false)
      (`self.SetActorEnableCollision` false)
      (`self.Change Zombie Mouth` true)
      (set `self.IsDead` true)
      (`self.Increase Points`)
      (`LightComponent.SetIntensity` (`self.TopLight`) (`self.Low Light Intensity`))
      (`self.Set Front Back Lights Intensity` 0.0)
      (if (`|EnumEquality` (`self.Zombie Type`) "NewEnumerator5")
        (`ActorComponent.K2_DestroyComponent` (`self.CapsuleDog`))
        (else
          (`ActorComponent.K2_DestroyComponent` (`self.CapsuleZombie`))))
      (`SceneComponent.SetVisibility` _decal true false)
      (`DecalComponent.SetDecalMaterial` _decal (`|GetArrayItem` (`self.Blood Decals`) (`KismetMathLibrary.RandomIntegerInRange` 0 9)))
      (else
        (set `self.IsDetected` true)
        (`self.FlashRed`)))
    (elif (`self.ActorHasTag` OtherActor "Tag_Projectile_Pistol")
      (set `self.ZombieHealth` (- (`self.ZombieHealth`) 50.0))
      (goto _label_2)
      (elif (`self.ActorHasTag` OtherActor "Tag_Projectile_Shotgun")
        (set `self.ZombieHealth` (- (`self.ZombieHealth`) 100.0))
        (goto _label_3)))))

(event `FlashRed`
  ;[1 1 1] Bullets Hits Zombie
  (`LightComponent.SetLightColor` (`self.FrontLight`) (struct :`R` 0.26652 :`G` 0.006296 :`B` 0.006296 :`A` 1.0) true)
  (`LightComponent.SetLightColor` (`self.BackLight`) (struct :`R` 0.26652 :`G` 0.006296 :`B` 0.006296 :`A` 1.0) true)
  (`self.Set Front Back Lights Intensity` (`self.Very High Light Intensity`))
  (`KismetSystemLibrary.Delay` 0.2)
  (`LightComponent.SetLightColor` (`self.FrontLight`) (struct :`R` 1.0 :`G` 1.0 :`B` 1.0 :`A` 1.0) true)
  (`LightComponent.SetLightColor` (`self.BackLight`) (struct :`R` 1.0 :`G` 1.0 :`B` 1.0 :`A` 1.0) true)
  (`self.Set Front Back Lights Intensity` (`self.Low Light Intensity`)))

(event `self.DetectedCollision.OnComponentBeginOverlap`
  (params (OverlappedComponent :type "PrimitiveComponent Object Reference") (OtherActor :type "Actor Object Reference") (OtherComp :type "PrimitiveComponent Object Reference") (OtherBodyIndex :type Integer) (bFromSweep :type Boolean) (SweepResult :type "HitResult Structure (by ref)"))
  ;[1 1 1] Detect player
  (if (`self.ActorHasTag` OtherActor "Tag_Player")
    (set `self.IsDetected` true)))

(fn `Change Zombie Mouth`
  (params (Random :type Boolean) (Grin :type Boolean) (`Open Mouth` :type Boolean))
  (bind _mesh (`self.Mesh`))
  (bind _mesh_2 (`self.Mesh`))
  (if (`|EnumInequality` (`self.Zombie Type`) "NewEnumerator5")
    (if (`self.MouthEnabled`)
      (if Random
        (`SkeletalMeshComponent.SetMorphTarget` _mesh "ZombieGrin" (`KismetMathLibrary.Conv_IntToDouble` (`KismetMathLibrary.RandomIntegerInRange` 0 1)) true)
        (`SkeletalMeshComponent.SetMorphTarget` _mesh "ZombieOpenMouth" (`KismetMathLibrary.Conv_IntToDouble` (`KismetMathLibrary.RandomIntegerInRange` 0 1)) true)
        (else
          (if Grin
            (`SkeletalMeshComponent.SetMorphTarget` _mesh_2 "ZombieGrin" 1.0 true)
            (else
              (`SkeletalMeshComponent.SetMorphTarget` _mesh_2 "ZombieGrin" 0.0 true)))
          (if `Open Mouth`
            (`SkeletalMeshComponent.SetMorphTarget` (`self.Mesh`) "ZombieOpenMouth" 1.0 true)
            (else
              (`SkeletalMeshComponent.SetMorphTarget` (`self.Mesh`) "ZombieOpenMouth" 0.0 true))))))))

(fn `Increase Points`
  (switch `/Game/__MyContent_Rami/Enums/BP_ZombieTypes` (`self.Zombie Type`)
    (:`NewEnumerator0`
      (set `self.Score Points` 100))
    (:`NewEnumerator1`
      (set `self.Score Points` 200))
    (:`NewEnumerator2`
      (set `self.Score Points` 400 :!label _label))
    (:`NewEnumerator5`
      (goto _label)))
  (if (`self.Mini-Boss`)
    (set `self.Score Points` (* (`self.Score Points`) 2)))
  (bind _game_manager (`/Game/__MyContent_Rami/Blueprints/BP_FunctionLibrary.Get Game Manager`))
  (`/Game/__MyContent_Rami/Blueprints/BP_GameManager.Set Score` _game_manager (`self.Score Points`)))

(fn `Set Front Back Lights Color`
  (params (NewLightColor :type "LinearColor Structure"))
  (`LightComponent.SetLightColor` (`self.FrontLight`) NewLightColor true)
  (`LightComponent.SetLightColor` (`self.BackLight`) NewLightColor true))

(fn `Set Front Back Lights Intensity`
  (params (NewIntensity :type "Float (double-precision)"))
  (`LightComponent.SetIntensity` (`self.FrontLight`) NewIntensity)
  (`LightComponent.SetIntensity` (`self.BackLight`) NewIntensity))

(fn `Set Health`
  (params (ZombieHealth :type "Float (double-precision)"))
  (set `self.ZombieHealth` ZombieHealth))

(fn `Set Parameters`
  (params (`Zombie Type` :type "/Game/__MyContent_Rami/Enums/BP_ZombieTypes Enum" :default "NewEnumerator0") (`Mini-Boss` :type Boolean))
  (bind _mesh (`self.Mesh`))
  (bind _output_get (set `self.Zombie Type` `Zombie Type`))
  (bind _output_get_2 (set `self.Mini-Boss` `Mini-Boss`))
  (switch `/Game/__MyContent_Rami/Enums/BP_ZombieTypes` _output_get
    (:`NewEnumerator0`
      (`self.Set Speed` 500.0)
      (`self.Set Health` 100.0)
      (`SkeletalMeshComponent.SetAnimInstanceClass` _mesh "/Game/__MyContent_Rami/Animations/ZombieAnimation.ZombieAnimation_C" :!label _label)
      (`ActorComponent.K2_DestroyComponent` (`self.CapsuleDog`)))
    (:`NewEnumerator1`
      (`self.Set Speed` 350.0)
      (`self.Set Health` 200.0)
      (goto _label))
    (:`NewEnumerator2`
      (`self.Set Speed` 250.0)
      (`self.Set Health` 400.0)
      (goto _label))
    (:`NewEnumerator5`
      (`self.Set Speed` 500.0)
      (`self.Set Health` 400.0)
      (`SkeletalMeshComponent.SetAnimInstanceClass` _mesh "/Game/__MyContent_Rami/Animations/DogAnimation.DogAnimation_C")
      (`ActorComponent.K2_DestroyComponent` (`self.CapsuleZombie`))))
  (if _output_get_2
    (`SceneComponent.SetWorldScale3D` (`self.Mesh`) (1.5 1.5 1.5))
    (set `self.ZombieHealth` (* (`self.ZombieHealth`) 2.0))))

(fn `Set Skin`
  (params (NewMesh :type "SkeletalMesh Object Reference"))
  (`SkinnedMeshComponent.SetSkinnedAssetAndUpdate` (`self.Mesh`) NewMesh true))

(fn `Set Speed`
  (params (`Run Speed` :type "Float (double-precision)"))
  (set `CharacterMovementComponent.MaxWalkSpeed` `Run Speed` (`self.CharacterMovement`)))

(fn `UserConstructionScript`)