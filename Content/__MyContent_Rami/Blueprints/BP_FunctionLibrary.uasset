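; A Blueprint function library of global helpers for player access, game manager access and UI input control.
; Getters cast the first player character to BP_FirstPersonPlayer and fetch the GameManager held by BP_GameMode.
; Show Mouse switches cursor visibility and input mode between game only, UI only, or both.
; Hide UI sets every UserWidget instance, including nested ones, to hidden.
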(fn `Get Game Manager`
  (returns (`Game Manager` :type "/Game/__MyContent_Rami/Blueprints/BP_GameManager Object Reference"))
  (bind _asbp_game_mode (cast `/Game/__MyContent_Rami/Blueprints/BP_GameMode` (`GameplayStatics.GetGameMode` null)))
  (return (`/Game/__MyContent_Rami/Blueprints/BP_GameMode.Game Manager` _asbp_game_mode)))

(fn `Get Player`
  (returns (Player :type "/Game/__MyContent_Rami/Blueprints/Characters/BP_FirstPersonPlayer Object Reference"))
  (bind _asbp_first_person_player (cast `/Game/__MyContent_Rami/Blueprints/Characters/BP_FirstPersonPlayer` (`GameplayStatics.GetPlayerCharacter` null)))
  (return _asbp_first_person_player))

(fn `Hide UI`
  (bind _foundwidgets (`WidgetBlueprintLibrary.GetAllWidgetsOfClass` null "/Script/UMG.UserWidget" false))
  (for _array_element _foundwidgets
    (`Widget.SetVisibility` _array_element "Hidden")))

(fn `Show Mouse`
  (params (Visible :type "/Game/__MyContent_Rami/Blueprints/Enums/BP_MouseStates Enum" :default "NewEnumerator0"))
  (bind _returnvalue (`GameplayStatics.GetPlayerController` null))
  (bind _returnvalue_2 (`GameplayStatics.GetPlayerController` null))
  (switch `/Game/__MyContent_Rami/Blueprints/Enums/BP_MouseStates` Visible
    (:`NewEnumerator1`
      (set `PlayerController.bShowMouseCursor` false _returnvalue_2)
      (`WidgetBlueprintLibrary.SetInputMode_GameOnly` _returnvalue))
    (:`NewEnumerator0`
      (set `PlayerController.bShowMouseCursor` true _returnvalue_2)
      (`WidgetBlueprintLibrary.SetInputMode_UIOnlyEx` _returnvalue null))
    (:`NewEnumerator2`
      (set `PlayerController.bShowMouseCursor` true _returnvalue_2)
      (`WidgetBlueprintLibrary.SetInputMode_GameAndUIEx` _returnvalue null))))