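; Central game manager that owns the match state, countdown timer, score and player health and stamina.
; On BeginPlay it creates HUD, pause and game-over widgets and plays music, with SetState switching visibility, pause and mouse mode.
; Tick formats the countdown, which only sets a flag at zero, while depleted health triggers Game Over.
; Damage scales by enemy type and miniboss status, and pickups grant weapons, ammo, health, time or score.
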(event `self.ReceiveBeginPlay`
  ;[1 1 1] Init
  (`self.Create UI`)
  (`self.Set State` "NewEnumerator1")
  (`GameplayStatics.PlaySound2D` "/Game/__MyContent_Rami/Audio/Black_Ops_III_-_Damned.Black_Ops_III_-_Damned" 1.0 1.0 0.0 null null))

(event `self.ReceiveTick`
  (params (DeltaSeconds :type "Float (single-precision)"))
  (bind _returnvalue (`KismetMathLibrary.Round` (`self.Countdown Timer`)))
  ;[1 1 1] Timer
  (if (not (`self.Timer Ended`))
    (set `self.Countdown Timer` (- (`self.Countdown Timer`) DeltaSeconds))
    (set `self.Int Minutes` (/ _returnvalue 60))
    (set `self.Int Seconds` (mod _returnvalue 60))
    (if (and (< (`self.Int Seconds`) 10) (> (`self.Int Minutes`) 0))
      (set `self.Extra Zero` "0")
      (else
        (set `self.Extra Zero` "")))
    (if (== (`self.Int Minutes`) 0)
      (set `self.Text Minutes` "")
      (else
        (set `self.Text Minutes` (`KismetStringLibrary.Concat_StrStr` (`KismetStringLibrary.Conv_IntToString` (`self.Int Minutes`)) ":"))))
    (set `self.Timer Countdown Text` (`KismetStringLibrary.Concat_StrStr` (`self.Text Minutes`) (`self.Extra Zero`) (`KismetStringLibrary.Conv_IntToString` (`self.Int Seconds`))))
    (if (and (<= (`self.Int Seconds`) 0) (<= (`self.Int Minutes`) 0))
      (set `self.Timer Ended` true))))

(fn `Collect Pickup`
  (params (`Item Picked Up` :type "/Game/__MyContent_Rami/Blueprints/Enums/BP_ItemPickup Enum" :default "NewEnumerator0"))
  (switch `/Game/__MyContent_Rami/Blueprints/Enums/BP_ItemPickup` `Item Picked Up`
    (:`NewEnumerator1`
      (bind _player (`/Game/__MyContent_Rami/Blueprints/BP_FunctionLibrary.Get Player`))
      (set `/Game/__MyContent_Rami/Blueprints/Characters/BP_FirstPersonPlayer.HasPistol` true _player)
      (`/Game/__MyContent_Rami/Blueprints/Characters/BP_FirstPersonPlayer.EquipGun` _player "NewEnumerator3")
      (`/Game/__MyContent_Rami/Blueprints/Characters/BP_FirstPersonPlayer.ResetAmmo` _player true false false)
      (`self.Set Score` 1000 :!label _label))
    (:`NewEnumerator0`
      (bind _player_2 (`/Game/__MyContent_Rami/Blueprints/BP_FunctionLibrary.Get Player`))
      (set `/Game/__MyContent_Rami/Blueprints/Characters/BP_FirstPersonPlayer.HasAssaultRifle` true _player_2)
      (`/Game/__MyContent_Rami/Blueprints/Characters/BP_FirstPersonPlayer.EquipGun` _player_2 "NewEnumerator1")
      (`/Game/__MyContent_Rami/Blueprints/Characters/BP_FirstPersonPlayer.ResetAmmo` _player_2 false true false)
      (goto _label))
    (:`NewEnumerator2`
      (bind _player_3 (`/Game/__MyContent_Rami/Blueprints/BP_FunctionLibrary.Get Player`))
      (set `/Game/__MyContent_Rami/Blueprints/Characters/BP_FirstPersonPlayer.HasShotgun` true _player_3)
      (`/Game/__MyContent_Rami/Blueprints/Characters/BP_FirstPersonPlayer.EquipGun` _player_3 "NewEnumerator2")
      (`/Game/__MyContent_Rami/Blueprints/Characters/BP_FirstPersonPlayer.ResetAmmo` _player_3 false false true)
      (goto _label))
    (:`NewEnumerator3`
      (bind _player_4 (`/Game/__MyContent_Rami/Blueprints/BP_FunctionLibrary.Get Player`))
      (`/Game/__MyContent_Rami/Blueprints/Characters/BP_FirstPersonPlayer.ResetAmmo` _player_4 true true true))
    (:`NewEnumerator4`
      (`self.Set Player Health` 100.0))
    (:`NewEnumerator5`
      (set `self.Countdown Timer` 120.0)
      (`self.Set Score` 500))))

(fn `Create UI`
  (`|ExecutionSequence`
    (:`then_0`
      (bind _returnvalue (`|CreateWidget` "/Game/__MyContent_Rami/Blueprints/UI/BP_HUD.BP_HUD_C"))
      (bind _output_get (set `self.HUD Widget` _returnvalue))
      (`UserWidget.AddToViewport` _output_get 0))
    (:`then_1`
      (bind _returnvalue_2 (`|CreateWidget` "/Game/__MyContent_Rami/Blueprints/UI/BP_Paused.BP_Paused_C"))
      (bind _output_get_2 (set `self.Paused Widget` _returnvalue_2))
      (`UserWidget.AddToViewport` _output_get_2 0))
    (:`then_2`
      (bind _returnvalue_3 (`|CreateWidget` "/Game/__MyContent_Rami/Blueprints/UI/BP_GameOver.BP_GameOver_C"))
      (bind _output_get_3 (set `self.GameOver Widget` _returnvalue_3))
      (`UserWidget.AddToViewport` _output_get_3 0))))

(fn `Damage Player`
  (params (`Enemy Sizes` :type "/Game/__MyContent_Rami/Blueprints/Enums/BP_ZombieTypes Enum" :default "NewEnumerator1") (`Mini-Boss` :type Boolean))
  (if `Mini-Boss`
    (set `self.Boss Multiplier` 2.0)
    (else
      (set `self.Boss Multiplier` 1.0)))
  (switch `/Game/__MyContent_Rami/Blueprints/Enums/BP_ZombieTypes` `Enemy Sizes`
    (:`NewEnumerator0`
      (set `self.Damage Multiplier` 1.0))
    (:`NewEnumerator1`
      (set `self.Damage Multiplier` 2.0))
    (:`NewEnumerator2`
      (set `self.Damage Multiplier` 4.0 :!label _label))
    (:`NewEnumerator5`
      (goto _label)))
  (`self.Set Player Health` (* (`self.Damage Multiplier`) (`self.Boss Multiplier`) -0.5)))

(fn `Get Player Health`
  (returns (Health :type "Float (double-precision)"))
  (return (`self.Health`)))

(fn `Get Player Stamina`
  (returns (Stamina :type "Float (double-precision)"))
  (return (`self.Stamina`)))

(fn `Get Score`
  (returns (Score :type Integer))
  (return (`self.Score`)))

(fn `Get State`
  (returns (`Current Game State` :type "/Game/__MyContent_Rami/Blueprints/Enums/BP_GameStates Enum"))
  (return (`self.Current Game State`)))

(fn `Get Timer Countdown`
  (returns (`Timer Countdown Text` :type String))
  (return (`self.Timer Countdown Text`)))

(fn `RetryLevel`
  (bind _returnvalue (`GameplayStatics.GetCurrentLevelName` true))
  (`GameplayStatics.OpenLevel` (`KismetStringLibrary.Conv_StringToName` _returnvalue)))

(fn `Set Player Health`
  (params (`Delta Health` :type "Float (double-precision)"))
  (bind _returnvalue (+ `Delta Health` (`self.Health`)))
  (if (<= _returnvalue 0.0)
    (set `self.Health` 0.0)
    (`self.Set State` "NewEnumerator3")
    (elif (> _returnvalue 100.0)
      (set `self.Health` 100.0)
      (`self.Set Score` 500)
      (else
        (set `self.Health` _returnvalue)))))

(fn `Set Player Stamina`
  (params (`Delta Stamina` :type "Float (double-precision)"))
  (bind _returnvalue (+ `Delta Stamina` (`self.Stamina`)))
  (if (< _returnvalue 0.0)
    (set `self.Stamina` 0.0)
    (elif (> _returnvalue 100.0)
      (set `self.Stamina` 100.0)
      (else
        (set `self.Stamina` _returnvalue)))))

(fn `Set Score`
  (params (`Delta Score` :type Integer))
  (set `self.Score` (+ `Delta Score` (`self.Score`))))

(fn `Set State`
  (params (`New State` :type "/Game/__MyContent_Rami/Blueprints/Enums/BP_GameStates Enum" :default "NewEnumerator0"))
  (if (`|EnumInequality` `New State` (`self.Current Game State`))
    (`/Game/__MyContent_Rami/Blueprints/BP_FunctionLibrary.Hide UI`)
    (bind _output_get (set `self.Current Game State` `New State`))
    (switch `/Game/__MyContent_Rami/Blueprints/Enums/BP_GameStates` _output_get
      (:`NewEnumerator1`
        (`GameplayStatics.SetGamePaused` false)
        (`Widget.SetVisibility` (`self.HUD Widget`) "Visible")
        (`/Game/__MyContent_Rami/Blueprints/BP_FunctionLibrary.Show Mouse` "NewEnumerator1"))
      (:`NewEnumerator2`
        (`GameplayStatics.SetGamePaused` true)
        (`Widget.SetVisibility` (`self.Paused Widget`) "Visible")
        (`/Game/__MyContent_Rami/Blueprints/BP_FunctionLibrary.Show Mouse` "NewEnumerator2"))
      (:`NewEnumerator3`
        (`GameplayStatics.SetGamePaused` true)
        (`Widget.SetVisibility` (`self.GameOver Widget`) "Visible")
        (`/Game/__MyContent_Rami/Blueprints/BP_FunctionLibrary.Show Mouse` "NewEnumerator0")))))

(fn `UserConstructionScript`)