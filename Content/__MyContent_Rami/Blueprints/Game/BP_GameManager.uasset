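; Central game manager for a first-person shooter, owning game state, health, stamina, score, countdown timer and saving.
; BeginPlay creates menu widgets, then shows the title screen or, if the GameInstance flags SkipTitle, spawns and possesses the player and restores saved data.
; SetState switches UI, pause and mouse mode; death or timeout triggers Game Over.
; Pickups and size-scaled enemy damage feed the stats, and a single-slot SaveGame persists progress.
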(event `self.ReceiveBeginPlay`
  ;[1 1 1] Init
  (`self.Create UI`)
  (bind _asbp_game_instance (cast `/Game/__MyContent_Rami/Blueprints/Game/BP_GameInstance` (`GameplayStatics.GetGameInstance`)))
  (if (`/Game/__MyContent_Rami/Blueprints/Game/BP_GameInstance.SkipTitle` _asbp_game_instance)
    (`self.StartPlay`)
    (else
      (`self.Set State` "NewEnumerator0")
      (bind _returnvalue (`GameplayStatics.GetCurrentLevelName` true))
      (set `/Game/__MyContent_Rami/Blueprints/Game/BP_GameInstance.DefaultLevel` _returnvalue _asbp_game_instance))))

(event `StartPlay`
  ;[1 1 1] StartPlay
  (bind _outactors (`GameplayStatics.GetAllActorsOfClass` "/Game/BP_PlaceInWorld/BP_PlayerStart.BP_PlayerStart_C"))
  (bind _defaultsceneroot (`/Game/BP_PlaceInWorld/BP_PlayerStart.DefaultSceneRoot` (`|GetArrayItem` _outactors)))
  (bind _returnvalue (`|SpawnActorFromClass` "/Game/__MyContent_Rami/Blueprints/Characters/BP_FirstPersonPlayer.BP_FirstPersonPlayer_C" (`KismetMathLibrary.MakeTransform` (`SceneComponent.K2_GetComponentLocation` _defaultsceneroot) (`SceneComponent.K2_GetComponentRotation` _defaultsceneroot)) "Undefined" "OverrideRootScale" null null))
  (`Controller.Possess` (`GameplayStatics.GetPlayerController` 0) _returnvalue)
  (`self.Reset Countdown Timer`)
  (`/Game/__MyContent_Rami/Blueprints/Characters/BP_FirstPersonPlayer.ResetAmmo` (`/Game/__MyContent_Rami/Blueprints/Game/BP_FunctionLibrary.Get Player`) true true true)
  (`AudioComponent.Play` (`self.RunningMusic`) 0.0)
  (`self.LoadGameData`)
  (`self.Create HUD UI`)
  (`self.Set State` "NewEnumerator1"))

(event `self.ReceiveTick`
  (params (DeltaSeconds :type "Float (single-precision)"))
  (bind _returnvalue (`KismetMathLibrary.Round` (`self.Countdown Timer`)))
  ;[1 1 1] Timer
  (if (not (`self.Timer Ended`))
    (set `self.Countdown Timer` (- (`self.Countdown Timer`) DeltaSeconds))
    (set `self.Int Minutes` (/ _returnvalue 60))
    (set `self.Int Seconds` (mod _returnvalue 60))
    (if (and (< (`self.Int Seconds`) 10) (> (`self.Int Minutes`) 0))
      (set `self.Extra Zero` "0")
      (else
        (set `self.Extra Zero` "")))
    (if (== (`self.Int Minutes`) 0)
      (set `self.Text Minutes` "")
      (else
        (set `self.Text Minutes` (`KismetStringLibrary.Concat_StrStr` (`KismetStringLibrary.Conv_IntToString` (`self.Int Minutes`)) ":"))))
    (set `self.Timer Countdown Text` (`KismetStringLibrary.Concat_StrStr` (`self.Text Minutes`) (`self.Extra Zero`) (`KismetStringLibrary.Conv_IntToString` (`self.Int Seconds`))))
    (if (and (<= (`self.Int Seconds`) 0) (<= (`self.Int Minutes`) 0))
      (set `self.Timer Ended` true)
      (`self.Set State` "NewEnumerator3")
      (set `/Game/__MyContent_Rami/Blueprints/UI/BP_GameOver.GameOverText` "Times Up!" (`self.GameOver Widget`)))))

(event `DisplaySaving`
  ;[1 1 1] Saving Text
  (set `self.Saving Text` "Saving...")
  (`KismetSystemLibrary.Delay` 2.0)
  (set `self.Saving Text` ""))

(fn `CheckGameSave`
  (returns (ReturnValue :type Boolean))
  (bind _returnvalue (`GameplayStatics.DoesSaveGameExist` (`self.SaveSlotName`)))
  (return _returnvalue))

(fn `Collect Pickup`
  (params (`Item Picked Up` :type "/Game/__MyContent_Rami/Blueprints/Enums/BP_ItemPickup Enum" :default "NewEnumerator0"))
  (bind _player (`/Game/__MyContent_Rami/Blueprints/Game/BP_FunctionLibrary.Get Player`))
  (bind _player_2 (`/Game/__MyContent_Rami/Blueprints/Game/BP_FunctionLibrary.Get Player`))
  (bind _player_3 (`/Game/__MyContent_Rami/Blueprints/Game/BP_FunctionLibrary.Get Player`))
  (switch `/Game/__MyContent_Rami/Blueprints/Enums/BP_ItemPickup` `Item Picked Up`
    (:`NewEnumerator1`
      (`/Game/__MyContent_Rami/Blueprints/Characters/BP_FirstPersonPlayer.Has Weapon` _player_3 "NewEnumerator3")
      (`/Game/__MyContent_Rami/Blueprints/Characters/BP_FirstPersonPlayer.EquipGun` _player_3 "NewEnumerator3")
      (`/Game/__MyContent_Rami/Blueprints/Characters/BP_FirstPersonPlayer.ResetAmmo` _player_3 true false false)
      (`self.Set Score` 1000 :!label _label))
    (:`NewEnumerator0`
      (`/Game/__MyContent_Rami/Blueprints/Characters/BP_FirstPersonPlayer.Has Weapon` _player_2 "NewEnumerator1")
      (`/Game/__MyContent_Rami/Blueprints/Characters/BP_FirstPersonPlayer.EquipGun` _player_2 "NewEnumerator1")
      (`/Game/__MyContent_Rami/Blueprints/Characters/BP_FirstPersonPlayer.ResetAmmo` _player_2 false true false)
      (goto _label))
    (:`NewEnumerator2`
      (`/Game/__MyContent_Rami/Blueprints/Characters/BP_FirstPersonPlayer.Has Weapon` _player "NewEnumerator2")
      (`/Game/__MyContent_Rami/Blueprints/Characters/BP_FirstPersonPlayer.EquipGun` _player "NewEnumerator2")
      (`/Game/__MyContent_Rami/Blueprints/Characters/BP_FirstPersonPlayer.ResetAmmo` _player false false true)
      (goto _label))
    (:`NewEnumerator3`
      (`/Game/__MyContent_Rami/Blueprints/Characters/BP_FirstPersonPlayer.ResetAmmo` (`/Game/__MyContent_Rami/Blueprints/Game/BP_FunctionLibrary.Get Player`) true true true)
      (`self.Set Score` 500 :!label _label_2))
    (:`NewEnumerator4`
      (`self.Set Player Health` 100.0)
      (`self.Set Player Stamina` 100.0))
    (:`NewEnumerator5`
      (`self.Reset Countdown Timer`)
      (goto _label_2))
    (:`NewEnumerator6`
      (`/Game/__MyContent_Rami/Blueprints/Characters/BP_FirstPersonPlayer.Set Key` (`/Game/__MyContent_Rami/Blueprints/Game/BP_FunctionLibrary.Get Player`) true)
      (`self.Set Score` 2000))))

(fn `Create HUD UI`
  (bind _returnvalue (`|CreateWidget` "/Game/__MyContent_Rami/Blueprints/UI/BP_HUD.BP_HUD_C"))
  (bind _output_get (set `self.HUD Widget` _returnvalue))
  (`UserWidget.AddToViewport` _output_get 0))

(fn `Create UI`
  (`|ExecutionSequence`
    (:`then_0`
      (bind _returnvalue (`|CreateWidget` "/Game/__MyContent_Rami/Blueprints/UI/BP_Paused.BP_Paused_C"))
      (bind _output_get (set `self.Paused Widget` _returnvalue))
      (`UserWidget.AddToViewport` _output_get 0))
    (:`then_1`
      (bind _returnvalue_2 (`|CreateWidget` "/Game/__MyContent_Rami/Blueprints/UI/BP_GameOver.BP_GameOver_C"))
      (bind _output_get_2 (set `self.GameOver Widget` _returnvalue_2))
      (`UserWidget.AddToViewport` _output_get_2 0))
    (:`then_2`
      (bind _returnvalue_3 (`|CreateWidget` "/Game/__MyContent_Rami/Blueprints/UI/BP_Won.BP_Won_C"))
      (bind _output_get_3 (set `self.Won Widget` _returnvalue_3))
      (`UserWidget.AddToViewport` _output_get_3 0))
    (:`then_3`
      (bind _returnvalue_4 (`|CreateWidget` "/Game/__MyContent_Rami/Blueprints/UI/BP_TitleScreen.BP_TitleScreen_C"))
      (bind _output_get_4 (set `self.Title Screen` _returnvalue_4))
      (`UserWidget.AddToViewport` _output_get_4 0))))

(fn `Damage Player`
  (params (`Enemy Sizes` :type "/Game/__MyContent_Rami/Blueprints/Enums/BP_ZombieTypes Enum" :default "NewEnumerator1") (`Mini-Boss` :type Boolean))
  (if `Mini-Boss`
    (set `self.Boss Multiplier` 2.0)
    (else
      (set `self.Boss Multiplier` 1.0)))
  (switch `/Game/__MyContent_Rami/Blueprints/Enums/BP_ZombieTypes` `Enemy Sizes`
    (:`NewEnumerator0`
      (set `self.Damage Multiplier` 1.0))
    (:`NewEnumerator1`
      (set `self.Damage Multiplier` 2.0))
    (:`NewEnumerator2`
      (set `self.Damage Multiplier` 4.0 :!label _label))
    (:`NewEnumerator5`
      (goto _label)))
  (`self.Set Player Health` (* (`self.Damage Multiplier`) (`self.Boss Multiplier`) -0.5)))

(fn `DeleteGameLevel`
  (bind _saveslotname (`self.SaveSlotName`))
  (bind _returnvalue (`GameplayStatics.DoesSaveGameExist` _saveslotname))
  (if _returnvalue
    (`GameplayStatics.DeleteGameInSlot` _saveslotname)))

(fn `Get Player Health`
  (returns (Health :type "Float (double-precision)"))
  (return (`self.Health`)))

(fn `Get Player Stamina`
  (returns (Stamina :type "Float (double-precision)"))
  (return (`self.Stamina`)))

(fn `Get Score`
  (returns (Score :type Integer))
  (return (`self.Score`)))

(fn `Get State`
  (returns (`Current Game State` :type "/Game/__MyContent_Rami/Blueprints/Enums/BP_GameStates Enum"))
  (return (`self.Current Game State`)))

(fn `Get Timer Countdown`
  (returns (`Timer Countdown Text` :type String))
  (return (`self.Timer Countdown Text`)))

(fn `GetSavingText`
  (returns (`Saving Text` :type String))
  (return (`self.Saving Text`)))

(fn `LoadGameData`
  (bind _saveslotname (`self.SaveSlotName`))
  (bind _returnvalue (`GameplayStatics.DoesSaveGameExist` _saveslotname))
  (if _returnvalue
    (bind _returnvalue_2 (`GameplayStatics.LoadGameFromSlot` _saveslotname))
    (bind _asbp_save_game (cast `/Game/__MyContent_Rami/Blueprints/Game/BP_SaveGame` _returnvalue_2))
    (`self.K2_SetActorLocation` (`/Game/__MyContent_Rami/Blueprints/Game/BP_FunctionLibrary.Get Player`) (`/Game/__MyContent_Rami/Blueprints/Game/BP_SaveGame.PlayerLocation` _asbp_save_game) false false)
    (set `self.Score` (`/Game/__MyContent_Rami/Blueprints/Game/BP_SaveGame.Score` _asbp_save_game))
    (`/Game/__MyContent_Rami/Blueprints/Characters/BP_FirstPersonPlayer.SetSaveParaments` (`/Game/__MyContent_Rami/Blueprints/Game/BP_FunctionLibrary.Get Player`) (`/Game/__MyContent_Rami/Blueprints/Game/BP_SaveGame.HasPistol` _asbp_save_game) (`/Game/__MyContent_Rami/Blueprints/Game/BP_SaveGame.HasRifle` _asbp_save_game) (`/Game/__MyContent_Rami/Blueprints/Game/BP_SaveGame.HasShotgun` _asbp_save_game) (`/Game/__MyContent_Rami/Blueprints/Game/BP_SaveGame.HasKey` _asbp_save_game) (`/Game/__MyContent_Rami/Blueprints/Game/BP_SaveGame.CurrentWeapon` _asbp_save_game) (`/Game/__MyContent_Rami/Blueprints/Game/BP_SaveGame.SaveCheckpoint` _asbp_save_game))))

(fn `LoadGameLevel`
  (bind _saveslotname (`self.SaveSlotName`))
  (bind _asbp_game_instance (cast `/Game/__MyContent_Rami/Blueprints/Game/BP_GameInstance` (`GameplayStatics.GetGameInstance`)))
  (set `/Game/__MyContent_Rami/Blueprints/Game/BP_GameInstance.SkipTitle` true _asbp_game_instance)
  (bind _returnvalue (`GameplayStatics.DoesSaveGameExist` _saveslotname))
  (if _returnvalue
    (bind _returnvalue_2 (`GameplayStatics.LoadGameFromSlot` _saveslotname))
    (bind _asbp_save_game (cast `/Game/__MyContent_Rami/Blueprints/Game/BP_SaveGame` _returnvalue_2))
    (`GameplayStatics.OpenLevel` (`KismetStringLibrary.Conv_StringToName` (`/Game/__MyContent_Rami/Blueprints/Game/BP_SaveGame.LevelName` _asbp_save_game)))
    (else
      (bind _asbp_game_instance_2 (cast `/Game/__MyContent_Rami/Blueprints/Game/BP_GameInstance` (`GameplayStatics.GetGameInstance`)))
      (`GameplayStatics.OpenLevel` (`KismetStringLibrary.Conv_StringToName` (`/Game/__MyContent_Rami/Blueprints/Game/BP_GameInstance.DefaultLevel` _asbp_game_instance_2))))))

(fn `Reset Countdown Timer`
  (set `self.Countdown Timer` 120.0))

(fn `SaveGame`
  (bind (_haskey _haspistol _hasassaultrifle _hasshotgun _currentweapon _savecheckpoint) (`/Game/__MyContent_Rami/Blueprints/Characters/BP_FirstPersonPlayer.GetSaveParameters` (`/Game/__MyContent_Rami/Blueprints/Game/BP_FunctionLibrary.Get Player`)))
  (`self.DisplaySaving`)
  (bind _returnvalue (`GameplayStatics.CreateSaveGameObject` "/Game/__MyContent_Rami/Blueprints/Game/BP_SaveGame.BP_SaveGame_C"))
  (bind _output_get (set `self.SaveGameInstance` _returnvalue))
  (set `/Game/__MyContent_Rami/Blueprints/Game/BP_SaveGame.Score` (`self.Score`) _output_get)
  (set `/Game/__MyContent_Rami/Blueprints/Game/BP_SaveGame.PlayerLocation` (`self.K2_GetActorLocation` (`/Game/__MyContent_Rami/Blueprints/Game/BP_FunctionLibrary.Get Player`)) _output_get)
  (bind _returnvalue_2 (`GameplayStatics.GetCurrentLevelName` true))
  (set `/Game/__MyContent_Rami/Blueprints/Game/BP_SaveGame.LevelName` _returnvalue_2 _output_get)
  (set `/Game/__MyContent_Rami/Blueprints/Game/BP_SaveGame.HasPistol` _haspistol _output_get)
  (set `/Game/__MyContent_Rami/Blueprints/Game/BP_SaveGame.HasRifle` _hasassaultrifle _output_get)
  (set `/Game/__MyContent_Rami/Blueprints/Game/BP_SaveGame.HasShotgun` _hasshotgun _output_get)
  (set `/Game/__MyContent_Rami/Blueprints/Game/BP_SaveGame.HasKey` _haskey _output_get)
  (set `/Game/__MyContent_Rami/Blueprints/Game/BP_SaveGame.CurrentWeapon` _currentweapon _output_get)
  (set `/Game/__MyContent_Rami/Blueprints/Game/BP_SaveGame.SaveCheckpoint` _savecheckpoint _output_get)
  (`GameplayStatics.SaveGameToSlot` _output_get (`/Game/__MyContent_Rami/Blueprints/Game/BP_SaveGame.SaveSlotName` _output_get) (`/Game/__MyContent_Rami/Blueprints/Game/BP_SaveGame.UserIndex` _output_get)))

(fn `Set Player Health`
  (params (`Delta Health` :type "Float (double-precision)"))
  (bind _returnvalue (+ `Delta Health` (`self.Health`)))
  (if (<= _returnvalue 0.0)
    (set `self.Health` 0.0)
    (`self.Set State` "NewEnumerator3")
    (set `/Game/__MyContent_Rami/Blueprints/UI/BP_GameOver.GameOverText` "You Died" (`self.GameOver Widget`))
    (elif (> _returnvalue 100.0)
      (set `self.Health` 100.0)
      (`self.Set Score` 500)
      (else
        (set `self.Health` _returnvalue)))))

(fn `Set Player Stamina`
  (params (`Delta Stamina` :type "Float (double-precision)"))
  (bind _returnvalue (+ `Delta Stamina` (`self.Stamina`)))
  (if (< _returnvalue 0.0)
    (set `self.Stamina` 0.0)
    (elif (> _returnvalue 100.0)
      (set `self.Stamina` 100.0)
      (else
        (set `self.Stamina` _returnvalue)))))

(fn `Set Score`
  (params (`Delta Score` :type Integer))
  (set `self.Score` (+ `Delta Score` (`self.Score`)))
  (if (< (`self.Score`) 0)
    (set `self.Score` 0)))

(fn `Set State`
  (params (`New State` :type "/Game/__MyContent_Rami/Blueprints/Enums/BP_GameStates Enum" :default "NewEnumerator0"))
  (`/Game/__MyContent_Rami/Blueprints/Game/BP_FunctionLibrary.Hide UI`)
  (bind _output_get (set `self.Current Game State` `New State`))
  (switch `/Game/__MyContent_Rami/Blueprints/Enums/BP_GameStates` _output_get
    (:`NewEnumerator1`
      (`GameplayStatics.SetGamePaused` false)
      (`Widget.SetVisibility` (`self.HUD Widget`) "Visible")
      (`/Game/__MyContent_Rami/Blueprints/Game/BP_FunctionLibrary.Show Mouse` "NewEnumerator1"))
    (:`NewEnumerator2`
      (`GameplayStatics.SetGamePaused` true)
      (`Widget.SetVisibility` (`self.Paused Widget`) "Visible")
      (`/Game/__MyContent_Rami/Blueprints/Game/BP_FunctionLibrary.Show Mouse` "NewEnumerator2"))
    (:`NewEnumerator0`
      (`GameplayStatics.SetGamePaused` true)
      (`Widget.SetVisibility` (`self.Title Screen`) "Visible")
      (`/Game/__MyContent_Rami/Blueprints/Game/BP_FunctionLibrary.Show Mouse` "NewEnumerator0"))
    (:`NewEnumerator3`
      (`GameplayStatics.SetGamePaused` true)
      (`Widget.SetVisibility` (`self.GameOver Widget`) "Visible")
      (`/Game/__MyContent_Rami/Blueprints/Game/BP_FunctionLibrary.Show Mouse` "NewEnumerator0"))
    (:`NewEnumerator4`
      (`GameplayStatics.SetGamePaused` true)
      (`Widget.SetVisibility` (`self.Won Widget`) "Visible")
      (`/Game/__MyContent_Rami/Blueprints/Game/BP_FunctionLibrary.Show Mouse` "NewEnumerator0"))))

(fn `UserConstructionScript`)