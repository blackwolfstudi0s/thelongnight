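; Zombie enemy character that chases and attacks the player, configured as Skinny, Average, Fat or Dog, optionally a scaled-up MiniBoss.
; A looping timer issues AI move orders once the player is detected by proximity or gunfire.
; Tagged projectiles reduce health and flash the lights red; death removes collision and shows a random blood decal.
; Attack overlap repeatedly damages the player through GameManager, while another overlap dims the zombie's lights near the player.
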(event `self.ReceiveBeginPlay`
  ;[1 1 1] Detour AI Controller
  (`self.Set Light Intensity` (`self.High Light Intensity`))
  (`KismetSystemLibrary.K2_SetTimer` null "TrackPlayer" 0.1 true))

(event `TrackPlayer`
  ;[1 1 1] Detour AI Controller
  (if (and (`self.IsDetected`) (not (`self.IsDead`)) (not (`self.IsAttacking`)))
    (bind _player (`/Game/__MyContent_Rami/Blueprints/BP_FunctionLibrary.Get Player`))
    (`AIController.MoveToLocation` (`AIBlueprintHelperLibrary.GetAIController` self) (`SceneComponent.K2_GetComponentLocation` (`Actor.RootComponent` _player)) 5.0 false true false true null false)))

(event `self.Mesh.OnComponentBeginOverlap`
  (params (OverlappedComponent :type "PrimitiveComponent Object Reference") (OtherActor :type "Actor Object Reference") (OtherComp :type "PrimitiveComponent Object Reference") (OtherBodyIndex :type Integer) (bFromSweep :type Boolean) (SweepResult :type "HitResult Structure (by ref)"))
  (bind _decal (`self.Decal`))
  ;[1 1 1] Bullets Hits Zombie
  (if (`self.ActorHasTag` OtherActor "Tag_Projectile_Rifle")
    (set `self.ZombieHealth` (- (`self.ZombieHealth`) 20.0))
    (`self.K2_DestroyActor` OtherActor :!label _label)
    (`self.FlashRed` :!label _label_2)
    (if (<= (`self.ZombieHealth`) 0.0)
      (set `self.IsDead` true)
      (`self.SetActorEnableCollision` false)
      (`self.Set Light Intensity` (`self.Low Light Intensity`))
      (`ActorComponent.K2_DestroyComponent` (`self.AttackingCollision`))
      (`ActorComponent.K2_DestroyComponent` (`self.DetectedCollision`))
      (`ActorComponent.K2_DestroyComponent` (`self.LightCollision`))
      (if (`|EnumEquality` (`self.Zombie Type`) "NewEnumerator5")
        (`ActorComponent.K2_DestroyComponent` (`self.CapsuleDog`))
        (else
          (`ActorComponent.K2_DestroyComponent` (`self.CapsuleZombie`))))
      (`SceneComponent.SetVisibility` _decal true false)
      (`DecalComponent.SetDecalMaterial` _decal (`|GetArrayItem` (`self.Blood Decals`) (`KismetMathLibrary.RandomIntegerInRange` 0 9)))
      (else
        (set `self.IsDetected` true)))
    (elif (`self.ActorHasTag` OtherActor "Tag_Projectile_Pistol")
      (set `self.ZombieHealth` (- (`self.ZombieHealth`) 50.0))
      (goto _label)
      (elif (`self.ActorHasTag` OtherActor "Tag_Projectile_Shotgun")
        (set `self.ZombieHealth` (- (`self.ZombieHealth`) 100.0))
        (goto _label_2)))))

(event `FlashRed`
  ;[1 1 1] Bullets Hits Zombie
  (`LightComponent.SetLightColor` (`self.FrontLight`) (struct :`R` 0.419108 :`A` 1.0) true)
  (`LightComponent.SetLightColor` (`self.BackLight`) (struct :`R` 0.419108 :`A` 1.0) true)
  (`self.Set Light Intensity` (`self.Very High Light Intensity`))
  (`KismetSystemLibrary.Delay` 0.3)
  (`LightComponent.SetLightColor` (`self.FrontLight`) (struct :`R` 1.0 :`G` 1.0 :`B` 1.0 :`A` 1.0) true)
  (`LightComponent.SetLightColor` (`self.BackLight`) (struct :`R` 1.0 :`G` 1.0 :`B` 1.0 :`A` 1.0) true)
  (`self.Set Light Intensity` (`self.High Light Intensity`)))

(event `self.AttackingCollision.OnComponentBeginOverlap`
  (params (OverlappedComponent :type "PrimitiveComponent Object Reference") (OtherActor :type "Actor Object Reference") (OtherComp :type "PrimitiveComponent Object Reference") (OtherBodyIndex :type Integer) (bFromSweep :type Boolean) (SweepResult :type "HitResult Structure (by ref)"))
  ;[1 1 1] Attacking
  (if (`self.ActorHasTag` OtherActor "Player")
    (bind _output_get (set `self.IsAttacking` true))
    (if _output_get :!label _label_3
      (bind _game_manager (`/Game/__MyContent_Rami/Blueprints/BP_FunctionLibrary.Get Game Manager`))
      (`/Game/__MyContent_Rami/Blueprints/BP_GameManager.Damage Player` _game_manager (`self.Zombie Type`) (`self.Mini-Boss`))
      (`KismetSystemLibrary.Delay` 0.25)
      (goto _label_3))))

(event `self.AttackingCollision.OnComponentEndOverlap`
  (params (OverlappedComponent :type "PrimitiveComponent Object Reference") (OtherActor :type "Actor Object Reference") (OtherComp :type "PrimitiveComponent Object Reference") (OtherBodyIndex :type Integer))
  ;[1 1 1] Attacking
  (if (`self.ActorHasTag` OtherActor "Player")
    (set `self.IsAttacking` false)))

(event `self.DetectedCollision.OnComponentBeginOverlap`
  (params (OverlappedComponent :type "PrimitiveComponent Object Reference") (OtherActor :type "Actor Object Reference") (OtherComp :type "PrimitiveComponent Object Reference") (OtherBodyIndex :type Integer) (bFromSweep :type Boolean) (SweepResult :type "HitResult Structure (by ref)"))
  (if (`self.ActorHasTag` OtherActor "Player")
    (set `self.IsDetected` true)))

(event `self.LightCollision.OnComponentBeginOverlap`
  (params (OverlappedComponent :type "PrimitiveComponent Object Reference") (OtherActor :type "Actor Object Reference") (OtherComp :type "PrimitiveComponent Object Reference") (OtherBodyIndex :type Integer) (bFromSweep :type Boolean) (SweepResult :type "HitResult Structure (by ref)"))
  ;[1 1 1] Lighting
  (bind _player (`/Game/__MyContent_Rami/Blueprints/BP_FunctionLibrary.Get Player`))
  (if (== _player OtherActor)
    (`self.Set Light Intensity` (`self.Low Light Intensity`))))

(event `self.LightCollision.OnComponentEndOverlap`
  (params (OverlappedComponent :type "PrimitiveComponent Object Reference") (OtherActor :type "Actor Object Reference") (OtherComp :type "PrimitiveComponent Object Reference") (OtherBodyIndex :type Integer))
  ;[1 1 1] Lighting
  (bind _player (`/Game/__MyContent_Rami/Blueprints/BP_FunctionLibrary.Get Player`))
  (if (== _player OtherActor)
    (`self.Set Light Intensity` (`self.High Light Intensity`))))

(fn `Set Health`
  (params (ZombieHealth :type "Float (double-precision)"))
  (set `self.ZombieHealth` ZombieHealth))

(fn `Set Light Colour`
  (params (NewLightColor :type "LinearColor Structure"))
  (`LightComponent.SetLightColor` (`self.FrontLight`) NewLightColor true)
  (`LightComponent.SetLightColor` (`self.BackLight`) NewLightColor true))

(fn `Set Light Intensity`
  (params (NewIntensity :type "Float (double-precision)"))
  (`LightComponent.SetIntensity` (`self.FrontLight`) NewIntensity)
  (`LightComponent.SetIntensity` (`self.BackLight`) NewIntensity))

(fn `Set Parameters`
  (params (`Zombie Type` :type "/Game/__MyContent_Rami/Blueprints/BP_ZombieTypes Enum" :default "NewEnumerator0") (`Mini-Boss` :type Boolean))
  (bind _mesh (`self.Mesh`))
  (bind _output_get (set `self.Zombie Type` `Zombie Type`))
  (bind _output_get_2 (set `self.Mini-Boss` `Mini-Boss`))
  (switch `/Game/__MyContent_Rami/Blueprints/BP_ZombieTypes` _output_get
    (:`NewEnumerator0`
      (`self.Set Speed` 500.0)
      (`self.Set Health` 100.0)
      (`SkeletalMeshComponent.SetAnimInstanceClass` _mesh "/Game/__MyContent_Rami/Blueprints/ZombieAnimation.ZombieAnimation_C" :!label _label)
      (`ActorComponent.K2_DestroyComponent` (`self.CapsuleDog`)))
    (:`NewEnumerator1`
      (`self.Set Speed` 350.0)
      (`self.Set Health` 200.0)
      (goto _label))
    (:`NewEnumerator2`
      (`self.Set Speed` 250.0)
      (`self.Set Health` 400.0)
      (goto _label))
    (:`NewEnumerator5`
      (`self.Set Speed` 500.0)
      (`self.Set Health` 400.0)
      (`SkeletalMeshComponent.SetAnimInstanceClass` _mesh "/Game/__MyContent_Rami/Blueprints/DogAnimation.DogAnimation_C")
      (`ActorComponent.K2_DestroyComponent` (`self.CapsuleZombie`))))
  (if _output_get_2
    (`SceneComponent.SetWorldScale3D` (`self.Mesh`) (1.5 1.5 1.5))
    (set `self.ZombieHealth` (* (`self.ZombieHealth`) 2.0))))

(fn `Set Skin`
  (params (NewMesh :type "SkeletalMesh Object Reference"))
  (`SkinnedMeshComponent.SetSkinnedAssetAndUpdate` (`self.Mesh`) NewMesh true))

(fn `Set Speed`
  (params (`Run Speed` :type "Float (double-precision)"))
  (set `CharacterMovementComponent.MaxWalkSpeed` `Run Speed` (`self.CharacterMovement`)))

(fn `UserConstructionScript`)