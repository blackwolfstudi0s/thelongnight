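; Explosive barrel actor that detonates once when a rifle, pistol or shotgun projectile, identified by actor tag, overlaps it.
; It plays an explosion sound and particle effect, then checks every actor overlapping its DamageRadius component.
; Zombies take heavy damage and award score, while the player takes damage and a score penalty through the game manager.
; The barrel destroys itself afterwards.
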(event `self.Explosive Barrel.OnComponentBeginOverlap`
  (params (OverlappedComponent :type "PrimitiveComponent Object Reference") (OtherActor :type "Actor Object Reference") (OtherComp :type "PrimitiveComponent Object Reference") (OtherBodyIndex :type Integer) (bFromSweep :type Boolean) (SweepResult :type "HitResult Structure (by ref)"))
  (bind _game_manager (`/Game/__MyContent_Rami/Blueprints/Game/BP_FunctionLibrary.Get Game Manager`))
  (bind _returnvalue (`self.K2_GetActorLocation`))
  (if (or (`self.ActorHasTag` OtherActor "Tag_Projectile_Rifle") (`self.ActorHasTag` OtherActor "Tag_Projectile_Pistol") (`self.ActorHasTag` OtherActor "Tag_Projectile_Shotgun"))
    (`/Engine/EditorBlueprintResources/StandardMacros.DoOnce` false
      (:`Completed`
        (`GameplayStatics.PlaySoundAtLocation` "/Game/StarterContent/Audio/Explosion01.Explosion01" _returnvalue (struct) 1.0 1.0 0.0 null null null)
        (`GameplayStatics.SpawnEmitterAtLocation` "/Game/__MyContent_Luke/_Lukes_content/MilitaryWeapDark/FX/P_RocketLauncher_Explosion_01.P_RocketLauncher_Explosion_01" _returnvalue (struct) (2.0 2.0 2.0))
        (for _array_element (`PrimitiveComponent.GetOverlappingActors` (`self.Damage Radius`) null)
          (if (`self.ActorHasTag` _array_element "Tag_Zombie")
            (bind _asbp_enemy_zombie (cast `/Game/__MyContent_Rami/Blueprints/Characters/BP_EnemyZombie` _array_element))
            (`/Game/__MyContent_Rami/Blueprints/Characters/BP_EnemyZombie.Set Health` _asbp_enemy_zombie -200.0)
            (`/Game/__MyContent_Rami/Blueprints/Game/BP_GameManager.Set Score` _game_manager 200)
            (elif (`self.ActorHasTag` _array_element "Tag_Player")
              (`/Game/__MyContent_Rami/Blueprints/Game/BP_GameManager.Set Player Health` _game_manager -50.0)
              (`/Game/__MyContent_Rami/Blueprints/Game/BP_GameManager.Set Score` _game_manager -1000))))
        (`self.K2_DestroyActor`)))))

(fn `UserConstructionScript`)