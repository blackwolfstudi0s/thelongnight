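; Proximity-driven door that swings open when the player comes within range and closes when they leave, with optional key locking.
; Tick polls player distance, showing a one-time find-key message through the game manager, or unlocking once and consuming the key.
; A timeline plays or reverses to lerp actor yaw from the initial door rotation captured at BeginPlay.
; The construction script picks one of two door meshes.
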(event `self.ReceiveBeginPlay`
  (bind (_returnvalue_roll _returnvalue_pitch _returnvalue_yaw) (`KismetMathLibrary.BreakRotator` (`SceneComponent.K2_GetComponentRotation` (`self.Door`))))
  (`SceneComponent.K2_AddRelativeRotation` (`self.Door`) (struct :`Yaw` -90.0) false false)
  (set `self.Initial Yaw` _returnvalue_yaw)
  (set `self.Initial Roll` _returnvalue_roll)
  (set `self.Initial Pitch` _returnvalue_pitch))

(event `self.ReceiveTick`
  (params (DeltaSeconds :type "Float (single-precision)"))
  (bind _player (`/Game/__MyContent_Rami/Blueprints/Game/BP_FunctionLibrary.Get Player`))
  (bind _locked (`self.Locked`))
  (bind _initial_roll (`self.Initial Roll`))
  (bind _initial_pitch (`self.Initial Pitch`))
  (bind _haskey (`/Game/__MyContent_Rami/Blueprints/Characters/BP_FirstPersonPlayer.GetKey` _player))
  (bind _returnvalue (<= (`self.GetDistanceTo` _player) (`self.DoorDistance`)))
  (if (and _returnvalue _locked (not _haskey))
    (`/Engine/EditorBlueprintResources/StandardMacros.DoOnce` false
      (:`Completed`
        (`/Game/__MyContent_Rami/Blueprints/Game/BP_GameManager.Set Display Text` (`/Game/__MyContent_Rami/Blueprints/Game/BP_FunctionLibrary.Get Game Manager`) "Find Key To Unlock Door")))
    (elif (and _returnvalue (or _haskey (not _locked)))
      (`|ExecutionSequence`
        (:`then_0`
          (`/Engine/EditorBlueprintResources/StandardMacros.DoOnce` false
            (:`Completed`
              (if (`self.Locked`)
                (set `self.Locked` false)
                (`/Game/__MyContent_Rami/Blueprints/Characters/BP_FirstPersonPlayer.Set Key` (`/Game/__MyContent_Rami/Blueprints/Game/BP_FunctionLibrary.Get Player`) false)))))
        (:`then_1`
          (bind (_direction _driver) (`Timeline|Door Driver` :!label _label)
            (:`Update`
              (`self.K2_SetActorRotation` (`KismetMathLibrary.RLerp` (`KismetMathLibrary.MakeRotator` _initial_roll _initial_pitch (`self.Initial Yaw`)) (`KismetMathLibrary.MakeRotator` _initial_roll _initial_pitch (+ (`self.Initial Yaw`) (`self.Yaw Open`))) _driver))))))
      (else
        (goto _label :!via `Reverse`)))))

(fn `UserConstructionScript`
  (bind _door (`self.Door`))
  (switch `/Game/__MyContent_Rami/Blueprints/Enums/BP_Doors` (`self.Door Selection`)
    (:`NewEnumerator0`
      (`StaticMeshComponent.SetStaticMesh` _door "/Game/ModularBuildingSet/Meshes/Store_fronts_doors/store_front_door_a_left.store_front_door_a_left"))
    (:`NewEnumerator2`
      (`StaticMeshComponent.SetStaticMesh` _door "/Game/ModularBuildingSet/Meshes/Store_fronts_doors/store_front_door_b_left.store_front_door_b_left")))
  (`SceneComponent.K2_AddRelativeRotation` _door (struct :`Yaw` 90.0) false false))