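; BP_NextLevel is a level-exit actor shown as a wolf that moves the game on when the player touches it.
; The construction script picks one of three wolf meshes from DogType.
; An overlap with an actor tagged Tag_Player passes a DoOnce, then calls the game manager to set a fixed score, save and load the next level, with short delays between steps.
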(event `self.SkeletalMesh.OnComponentBeginOverlap`
  (params (OverlappedComponent :type "PrimitiveComponent Object Reference") (OtherActor :type "Actor Object Reference") (OtherComp :type "PrimitiveComponent Object Reference") (OtherBodyIndex :type Integer) (bFromSweep :type Boolean) (SweepResult :type "HitResult Structure (by ref)"))
  (bind _game_manager (`/Game/__MyContent_Rami/Blueprints/Game/BP_FunctionLibrary.Get Game Manager`))
  (if (`self.ActorHasTag` OtherActor "Tag_Player")
    (`/Engine/EditorBlueprintResources/StandardMacros.DoOnce` false
      (:`Completed`
        (`KismetSystemLibrary.Delay` 0.1)
        (`/Game/__MyContent_Rami/Blueprints/Game/BP_GameManager.Set Score` _game_manager 2000)
        (`/Game/__MyContent_Rami/Blueprints/Game/BP_GameManager.SaveGame` _game_manager true)
        (`KismetSystemLibrary.Delay` 0.1)
        (`/Game/__MyContent_Rami/Blueprints/Game/BP_GameManager.LoadNextLevel` _game_manager)))))

(fn `UserConstructionScript`
  (bind _skeletalmesh (`self.SkeletalMesh`))
  (switch `/Game/__MyContent_Rami/Blueprints/Enums/BP_DogTypes` (`self.DogType`)
    (:`NewEnumerator0`
      (`SkinnedMeshComponent.SetSkinnedAssetAndUpdate` _skeletalmesh "/Game/__MyContent_Rami/Packs/ZombieMeshes/SK_Wolf_3.SK_Wolf_3" true))
    (:`NewEnumerator1`
      (`SkinnedMeshComponent.SetSkinnedAssetAndUpdate` _skeletalmesh "/Game/__MyContent_Rami/Packs/ZombieMeshes/SK_Wolf_2.SK_Wolf_2" true))
    (:`NewEnumerator2`
      (`SkinnedMeshComponent.SetSkinnedAssetAndUpdate` _skeletalmesh "/Game/__MyContent_Rami/Packs/ZombieMeshes/SK_Wolf_1.SK_Wolf_1" true))))