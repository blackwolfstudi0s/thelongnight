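; BP_CheckPoint is a checkpoint trigger that records the player's position in the "Check" save slot.
; On any Trigger overlap with Load enabled, it stores the first-person character's location and a load flag in BP_Save, reusing or creating the save.
; With Load disabled, it clears that flag in the existing save, so the same Blueprint can either set or cancel a checkpoint.
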(event `self.Trigger.OnComponentBeginOverlap`
  (params (OverlappedComponent :type "PrimitiveComponent Object Reference") (OtherActor :type "Actor Object Reference") (OtherComp :type "PrimitiveComponent Object Reference") (OtherBodyIndex :type Integer) (bFromSweep :type Boolean) (SweepResult :type "HitResult Structure (by ref)"))
  (bind _player_location (`self.Player Location`))
  (if (`self.Load`)
    (`|ExecutionSequence`
      (:`then_0`
        (bind _asfirst_person_character (cast `/Game/FirstPersonBP/Blueprints/FirstPersonCharacter` (`GameplayStatics.GetPlayerCharacter` 0)))
        (set `self.Player Location` (`self.K2_GetActorLocation` _asfirst_person_character)))
      (:`then_1`
        (bind _returnvalue (`GameplayStatics.DoesSaveGameExist` "Check"))
        (if _returnvalue
          (bind _returnvalue_2 (`GameplayStatics.LoadGameFromSlot` "Check"))
          (bind _asbp_save (cast `/Game/__MyContent_Ellani/Blueprints/BP_Save` _returnvalue_2))
          (set `/Game/__MyContent_Ellani/Blueprints/BP_Save.2 Player Location` _player_location _asbp_save)
          (set `/Game/__MyContent_Ellani/Blueprints/BP_Save.2 Load` true _asbp_save)
          (`GameplayStatics.SaveGameToSlot` _asbp_save "Check")
          (else
            (bind _returnvalue_3 (`GameplayStatics.CreateSaveGameObject` "/Game/__MyContent_Ellani/Blueprints/BP_Save.BP_Save_C"))
            (set `/Game/__MyContent_Ellani/Blueprints/BP_Save.2 Player Location` _player_location _returnvalue_3)
            (set `/Game/__MyContent_Ellani/Blueprints/BP_Save.2 Load` true _returnvalue_3)
            (`GameplayStatics.SaveGameToSlot` _returnvalue_3 "Check")))))
    (else
      (bind _returnvalue_4 (`GameplayStatics.LoadGameFromSlot` "Check"))
      (bind _asbp_save_2 (cast `/Game/__MyContent_Ellani/Blueprints/BP_Save` _returnvalue_4))
      (set `/Game/__MyContent_Ellani/Blueprints/BP_Save.2 Load` false _asbp_save_2)
      (`GameplayStatics.SaveGameToSlot` _asbp_save_2 "Check"))))

(fn `UserConstructionScript`)