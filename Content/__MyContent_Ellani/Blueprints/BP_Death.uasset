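; BP_Death is a death trigger volume that returns the player to the last saved checkpoint.
; Any overlap on its Trigger component disables first-person character input, without checking which actor overlapped.
; If the "Check" save slot exists, it loads BP_Save, moves the player to the stored location and re-enables input.
; With no save, it opens the level named by Level instead.
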(event `self.Trigger.OnComponentBeginOverlap`
  (params (OverlappedComponent :type "PrimitiveComponent Object Reference") (OtherActor :type "Actor Object Reference") (OtherComp :type "PrimitiveComponent Object Reference") (OtherBodyIndex :type Integer) (bFromSweep :type Boolean) (SweepResult :type "HitResult Structure (by ref)"))
  (bind _asfirst_person_character (cast `/Game/FirstPersonBP/Blueprints/FirstPersonCharacter` (`GameplayStatics.GetPlayerCharacter` 0)))
  (`self.DisableInput` _asfirst_person_character (`GameplayStatics.GetPlayerController` 0))
  (bind _returnvalue (`GameplayStatics.DoesSaveGameExist` "Check"))
  (if _returnvalue
    (bind _returnvalue_2 (`GameplayStatics.LoadGameFromSlot` "Check"))
    (bind _asbp_save (cast `/Game/__MyContent_Ellani/Blueprints/BP_Save` _returnvalue_2))
    (bind _asfirst_person_character_2 (cast `/Game/FirstPersonBP/Blueprints/FirstPersonCharacter` (`GameplayStatics.GetPlayerCharacter` 0)))
    (`self.K2_SetActorLocation` _asfirst_person_character_2 (`/Game/__MyContent_Ellani/Blueprints/BP_Save.2 Player Location` _asbp_save) false false)
    (`self.EnableInput` _asfirst_person_character_2 (`GameplayStatics.GetPlayerController` 0))
    (else
      (`GameplayStatics.OpenLevel` (`self.Level`)))))

(fn `UserConstructionScript`)